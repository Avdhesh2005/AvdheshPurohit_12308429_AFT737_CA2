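; Base tower actor, apparently for a tower defense game and still a work in progress.
; BeginPlay reads the BasicTower row of DT_TowerData and stores its base damage.
; Pressing P runs ShootTarget, which checks TargetEnemy and calls ApplyDamage without a damaged actor wired, printing debug messages.
; Range sphere sizing, fire rate, ability and async mesh loading are disconnected, and nothing here assigns TargetEnemy.
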(event EventBeginPlay
  (bind _returnvalue (Utilities|GetDataTableRow "/Game/Blueprints/DT_TowerData.DT_TowerData" "BasicTower")
    (:then
      (Variables|Default|SetCurrentDamage (.basedamage _returnvalue)))))

(event Input|KeyboardEvents|P
  (params (Key :type Key%20Structure :default "None"))
  (:Pressed
    (Development|PrintString "\"P is Pressed\"")
    (CallFunction|ShootTarget)))

(fn ConstructionScript)

(fn ShootTarget
  (Utilities|IsValid (Variables|Default|GetTargetEnemy)
    (:Is%20Valid
      (Game|Damage|ApplyDamage 0 (Variables|Default|GetCurrentDamage) 0 self)
      (Development|PrintString "Shot fired at enemy!"))
    (:Is%20Not%20Valid
      (Development|PrintString "Hello"))))