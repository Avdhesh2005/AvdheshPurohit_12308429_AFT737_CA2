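; BP_Enemy is an enemy actor that takes damage and is destroyed when its health runs out.
; The AnyDamage event subtracts damage from CurrentHealth and writes the new value to HealthText.
; At zero or below it prints a message and destroys the actor, otherwise it prints a placeholder debug string.
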(event Game|Damage|EventAnyDamage
  (params (Damage :type Float%20%28single-precision%29) (DamageType :type Damage%20Type%20Object%20Reference) (InstigatedBy :type Controller%20Object%20Reference) (DamageCauser :type Actor%20Object%20Reference))
  (Variables|Default|SetCurrentHealth (- (Variables|Default|GetCurrentHealth) Damage))
  (Rendering|Components|TextRender|SetText (Variables|Default|GetHealthText) (Utilities|Text|ToText(Float) (Variables|Default|GetCurrentHealth) "HalfToEven"))
  (if (<= (Variables|Default|GetCurrentHealth) 0.0)
    (Development|PrintString "Enemy++")
    (Actor|DestroyActor)
    (else
      (Development|PrintString "KJKJBGb"))))

(fn ConstructionScript)